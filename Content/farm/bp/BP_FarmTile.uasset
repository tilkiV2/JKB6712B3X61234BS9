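; Farm tile where the player plants wheat, corn or pumpkin seeds and harvests the grown crop.
; PlantSeed checks the held seed, plays a timed input-locking widget, and removes one seed from the SGK player inventory.
; Growth swaps static meshes through three stages, with GrowTime macro countdowns shown on Text3D.
; Activate harvests grown crops behind another widget, spawns loose produce (pumpkin's spawn class is unset) and resets the tile.
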(event Custom|PlantWheat
  (bind _relative_transformlocation (Variables|Default|GetRelative%20TransformLocation))
  (bind _returnvalue (AddComponent|AddStaticMeshComponent false (Math|Transform|MakeTransform _relative_transformlocation "0, 0, 0" "1,1,1")))
  (Utilities|GrowTime (Variables|Default|GetWheatGrowTime)
    (:Out
      (Components|DestroyComponent _returnvalue)
      (bind _returnvalue_2 (AddComponent|AddStaticMeshComponent false (Math|Transform|MakeTransform _relative_transformlocation "0, 0, 0" "1,1,1")))
      (Utilities|GrowTime (Variables|Default|GetWheatGrowTime)
        (:Out
          (Components|DestroyComponent _returnvalue_2)
          (bind _returnvalue_3 (AddComponent|AddStaticMeshComponent false (Math|Transform|MakeTransform _relative_transformlocation "0, 0, 0" "1,1,1")))
          (Variables|Default|SetFullyGrown? true)
          (Variables|Default|SetCurrentMesh _returnvalue_3)
          (Variables|Default|SetWhatCanBeHarvested "Wheat"))))))

(event Custom|PlantPumpkin
  (bind _relative_transformlocation (Variables|Default|GetRelative%20TransformLocation))
  (bind _returnvalue (AddComponent|AddStaticMeshComponent false (Math|Transform|MakeTransform _relative_transformlocation "0, 0, 0" "1,1,1")))
  (Utilities|GrowTime (Variables|Default|GetPumpkinGrowTime)
    (:Out
      (Components|DestroyComponent _returnvalue)
      (bind _returnvalue_2 (AddComponent|AddStaticMeshComponent false (Math|Transform|MakeTransform _relative_transformlocation "0, 0, 0" "1,1,1")))
      (Utilities|GrowTime (Variables|Default|GetPumpkinGrowTime)
        (:Out
          (Components|DestroyComponent _returnvalue_2)
          (bind _returnvalue_3 (AddComponent|AddStaticMeshComponent false (Math|Transform|MakeTransform _relative_transformlocation "0, 0, 0" "1,1,1")))
          (Variables|Default|SetFullyGrown? true)
          (Variables|Default|SetCurrentMesh _returnvalue_3)
          (Variables|Default|SetWhatCanBeHarvested "Pumpkin"))))))

(event Custom|PlantCorn
  (bind _relative_transformlocation (Variables|Default|GetRelative%20TransformLocation))
  (bind _returnvalue (AddComponent|AddStaticMeshComponent false (Math|Transform|MakeTransform _relative_transformlocation "0, 0, 0" "1,1,1")))
  (Utilities|GrowTime (Variables|Default|GetCornGrowTime)
    (:Out
      (Components|DestroyComponent _returnvalue)
      (bind _returnvalue_2 (AddComponent|AddStaticMeshComponent false (Math|Transform|MakeTransform _relative_transformlocation "0, 0, 0" "1,1,1")))
      (Utilities|GrowTime (Variables|Default|GetCornGrowTime)
        (:Out
          (Components|DestroyComponent _returnvalue_2)
          (bind _returnvalue_3 (AddComponent|AddStaticMeshComponent false (Math|Transform|MakeTransform _relative_transformlocation "0, 0, 0" "1,1,1")))
          (Variables|Default|SetFullyGrown? true)
          (Variables|Default|SetCurrentMesh _returnvalue_3)
          (Variables|Default|SetWhatCanBeHarvested "Corn"))))))

(event EventPlantSeed
  (if (Variables|Default|GetEkili_mi?)
    (Development|PrintString "false")
    (else
      (bind _asbp_sgkmaster_character (Utilities|Casting|CastToBP_SGKMasterCharacter (Game|GetPlayerCharacter 0)))
      ;[1 0 0.02781] Seed Elinde Mi ?
      (bind _returnvalue (Default|IsItemHeld (Variables|/Game/SurvivalGameKitV2/Blueprints/Characters/BP_SGKMasterCharacter.BP_SGKMasterCharacter_C|GetPlayerInventory _asbp_sgkmaster_character) "WheatSeed"))
      (if _returnvalue
        ;[1 0 0.02781] Ekme Witget'i
        (Utilities|PlantingWidget)
        ;[0 0 0] Bunu Tek bir makro haline getirebilirsin ilerde
        (Utilities|DoWeHaveWheatSeed
          (:output
            (CallFunction|PlantWheat)
            (Variables|Default|SetEkili_mi? true :!label _label)
            (Development|PrintString "ekti")))
        (else
          (bind _returnvalue_2 (Default|IsItemHeld (Variables|/Game/SurvivalGameKitV2/Blueprints/Characters/BP_SGKMasterCharacter.BP_SGKMasterCharacter_C|GetPlayerInventory _asbp_sgkmaster_character) "CornSeed"))
          (if _returnvalue_2
            (Utilities|PlantingWidget)
            (Utilities|DoWeHaveCornSeed
              (:output
                (CallFunction|PlantCorn)
                (goto _label)))
            (else
              (bind _returnvalue_3 (Default|IsItemHeld (Variables|/Game/SurvivalGameKitV2/Blueprints/Characters/BP_SGKMasterCharacter.BP_SGKMasterCharacter_C|GetPlayerInventory _asbp_sgkmaster_character) "PumpkinSeed"))
              (if _returnvalue_3
                (Utilities|PlantingWidget)
                (Utilities|DoWeHavePumpkinSeed
                  (:output
                    (CallFunction|PlantPumpkin)
                    (goto _label)))))))))))

(event EventBeginPlay
  (Class|Text3DComponent|SetText (Variables|Default|GetText3D) (Variables|Default|GetValue))
  (bind _asbp_sgkmaster_character (Utilities|Casting|CastToBP_SGKMasterCharacter (Game|GetPlayerCharacter 0)))
  (Variables|Default|Setkarakter _asbp_sgkmaster_character))

(event EventActivate
  (bind _returnvalue (Game|GetPlayerCharacter 0))
  (bind _returnvalue_2 (Game|GetPlayerController 0))
  (bind _text3d (Variables|Default|GetText3D))
  (bind _returnvalue_3 (Transformation|GetWorldLocation _text3d))
  (bind _returnvalue_4 (Math|Conversions|ToTransform(Vector) _returnvalue_3))
  (if (Variables|Default|GetFullyGrown?)
    (Input|DisableInput _returnvalue _returnvalue_2)
    (bind _returnvalue_5 (UserInterface|CreateWidget "/Game/farm/UI/UI_harvesting.UI_harvesting_C"))
    (bind _output_get (Variables|Default|SetWidget_ref_harvest _returnvalue_5))
    (UserInterface|Viewport|AddtoViewport _output_get 0)
    (UserInterface|Animation|PlayAnimation _returnvalue_5 (Variables|/Game/farm/UI/UI_harvesting.UI_harvesting_C|GetNewAnimation _returnvalue_5) 0.0 1 "Forward" 1.0 false)
    (Utilities|FlowControl|Delay 5.0)
    (Widget|RemovefromParent _returnvalue_5)
    (Input|EnableInput _returnvalue _returnvalue_2)
    (Components|DestroyComponent (Variables|Default|GetCurrentMesh))
    (switch string (Variables|Default|GetWhatCanBeHarvested)
      (:Default
        _)
      (:Wheat
        (Game|SpawnActorfromClass "/Game/SurvivalGameKitV2/Blueprints/Items/WorldItems/BP_WheatLoose.BP_WheatLoose_C" _returnvalue_4 "Undefined" 0 false false 0))
      (:Corn
        (Game|SpawnActorfromClass "/Game/SurvivalGameKitV2/Blueprints/Items/WorldItems/BP_BP_CornLoose.BP_BP_CornLoose_C" _returnvalue_4 "Undefined" 0 false false 0))
      (:Pumpkin
        (Game|SpawnActorfromClass "/Game/SurvivalGameKitV2/Blueprints/Items/WorldItems/PumpkinLoose.PumpkinLoose_C" _returnvalue_4 "Undefined" 0 false false 0)))
    (Variables|Default|SetFullyGrown? false)
    (Variables|Default|SetCurrentMesh 0)
    (Variables|Default|SetEkili_mi? false)
    (Variables|Default|SetEkili_mi? false)))

(fn ConstructionScript)